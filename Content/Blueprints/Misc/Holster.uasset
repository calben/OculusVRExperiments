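; Holster actor that snaps an overlapping AlienGun onto its Sphere2 component and records it as AttachedActor.
; Any other overlapping actor clears that reference without detaching and starts a one-second ActorJustRemoved lockout during which overlaps are ignored.
; A branch that would detach the held actor when BP_MotionControllerRight overlaps is present but disconnected, so it never runs.
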(event `self.ReceiveActorBeginOverlap`
  (params (OtherActor :type "Actor Object Reference"))
  (if (not (`self.ActorJustRemoved`))
    (bind _asalien_gun (cast `/Game/Blueprints/Weapons/AlienGun` OtherActor)
      (:`then`
        (`self.K2_AttachRootComponentTo` _asalien_gun (`self.Sphere2`) "None" "KeepRelativeOffset" true)
        (set `self.AttachedActor` _asalien_gun))
      (:`CastFailed`
        (set `self.AttachedActor` null)
        (set `self.ActorJustRemoved` true)
        (`KismetSystemLibrary.Delay` 1.0)
        (set `self.ActorJustRemoved` false)))))

(fn `UserConstructionScript`)