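; Bauble is a physics-driven actor that jostles around the level while staying loosely tethered to the player.
; Its static mesh receives a random horizontal force on BeginPlay and again whenever another actor overlaps its sphere.
; Each Tick, a mesh at least 2000 units from the player pawn is pulled back by a force that grows with distance.
; The recorded start time is not read anywhere in the graph.
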(event `self.ReceiveBeginPlay`
  (bind _returnvalue (`KismetMathLibrary.RandomIntegerInRange` -2 2))
  (bind (_startingforce_x _startingforce_y) (`KismetMathLibrary.BreakVector` (`self.StartingForce`)))
  (`|ExecutionSequence`
    (:`then_0`
      (set `self.T_start` (`KismetSystemLibrary.GetGameTimeInSeconds`))
      (set `self.StartingForce` (10000.0 10000.0 0.0)))
    (:`then_1`
      (`PrimitiveComponent.AddForce` (`self.StaticMesh`) (`KismetMathLibrary.MakeVector` (* _returnvalue _startingforce_x) (* _returnvalue _startingforce_y)) "None" false))))

(event `self.Sphere.OnComponentBeginOverlap`
  (params (OverlappedComponent :type "PrimitiveComponent Object Reference") (OtherActor :type "Actor Object Reference") (OtherComp :type "PrimitiveComponent Object Reference") (OtherBodyIndex :type Integer) (bFromSweep :type Boolean) (SweepResult :type "HitResult Structure (by ref)"))
  (bind _returnvalue (`KismetMathLibrary.RandomIntegerInRange` -2 2))
  (bind (_startingforce_x _startingforce_y) (`KismetMathLibrary.BreakVector` (`self.StartingForce`)))
  (if (!= OtherActor self)
    (`PrimitiveComponent.AddForce` (`self.StaticMesh`) (`KismetMathLibrary.MakeVector` (* _returnvalue _startingforce_x) (* _returnvalue _startingforce_y)) "None" false)))

(event `self.ReceiveTick`
  (params (DeltaSeconds :type "Float (single-precision)"))
  (bind _returnvalue (- (`self.K2_GetActorLocation` (`GameplayStatics.GetPlayerPawn` 0)) (`SceneComponent.K2_GetComponentLocation` (`self.StaticMesh`))))
  (if (>= (`KismetMathLibrary.VSize` _returnvalue) 2000.0)
    (`PrimitiveComponent.AddForce` (`self.StaticMesh`) (* _returnvalue 5) "None" false)))

(fn `UserConstructionScript`)