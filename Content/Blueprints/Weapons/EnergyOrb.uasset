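; EnergyOrb is a weapon actor that damages what its Box collider overlaps and then destroys itself.
; On overlap with any actor other than itself, it spawns a scaled-down ProjectileImpactBlast at the Orb component's location and rotation.
; It sends a fixed damage amount through a DamageActor message, so the orb needs no cast to the target's class.
; It also prints both actor names for debugging, and its graphs contain no movement logic.
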(event `self.Box.OnComponentBeginOverlap`
  (params (OverlappedComponent :type "PrimitiveComponent Object Reference") (OtherActor :type "Actor Object Reference") (OtherComp :type "PrimitiveComponent Object Reference") (OtherBodyIndex :type Integer) (bFromSweep :type Boolean) (SweepResult :type "HitResult Structure (by ref)"))
  (bind (_returnvalue_location _returnvalue_rotation) (`KismetMathLibrary.BreakTransform` (`SceneComponent.K2_GetComponentToWorld` (`self.Orb`))))
  (if (!= OtherActor self)
    (`|SpawnActorFromClass` "/Game/Blueprints/ProjectileImpactBlast.ProjectileImpactBlast_C" (`KismetMathLibrary.MakeTransform` _returnvalue_location _returnvalue_rotation (0.25 0.25 0.25)) "Undefined" "OverrideRootScale")
    (message `/Game/Blueprints/DamageInterface.DamageActor` OtherActor 10.0)
    (`KismetSystemLibrary.PrintString` (`KismetSystemLibrary.GetDisplayName` OtherActor))
    (`KismetSystemLibrary.PrintString` (`KismetSystemLibrary.GetDisplayName` self))
    (`self.K2_DestroyActor`)))

(fn `UserConstructionScript`)