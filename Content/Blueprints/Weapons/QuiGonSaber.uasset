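; QuiGonSaber is a grabbable lightsaber weapon with a Handle and a toggleable Blade.
; Pickup disables Handle physics and snaps it to the supplied component.
; An index press toggles Blade visibility once, with a DoOnce that resets on release.
; Drop enables physics and detaches, then after a short delay snaps the Handle to Holster3 on the TwoBrothersPawnTEMP player pawn and hides the Blade.
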(event `/Game/VirtualRealityBP/Blueprints/IndexInterface.IndexPressed`
  (`/Engine/EditorBlueprintResources/StandardMacros.DoOnce` false :!label _label
    (:`Completed`
      (`SceneComponent.ToggleVisibility` (`self.Blade`) false))))

(event `/Game/VirtualRealityBP/Blueprints/IndexInterface.IndexReleased`
  (goto _label :!via `Reset`))

(event `/Game/VirtualRealityBP/Blueprints/PickupActorInterface.Pickup`
  (params (AttachTo :type "SceneComponent Object Reference"))
  (bind _handle (`self.Handle`))
  (`self.K2_DetachFromActor` "KeepWorld" "KeepWorld")
  (`PrimitiveComponent.SetSimulatePhysics` _handle false)
  (`SceneComponent.K2_AttachToComponent` _handle AttachTo "None" "SnapToTarget" "SnapToTarget" "KeepRelative" true))

(event `/Game/VirtualRealityBP/Blueprints/PickupActorInterface.Drop`
  (`PrimitiveComponent.SetSimulatePhysics` (`self.Handle`) true)
  (`self.K2_DetachFromActor` "KeepWorld" "KeepWorld")
  (`KismetSystemLibrary.Delay` 0.2)
  (bind _astwo_brothers_pawn_temp (cast `/Game/VirtualRealityBP/Blueprints/TwoBrothersPawnTEMP` (`GameplayStatics.GetPlayerPawn` 0)))
  (`SceneComponent.K2_AttachToComponent` (`self.Handle`) (`/Game/VirtualRealityBP/Blueprints/TwoBrothersPawnTEMP.Holster3` _astwo_brothers_pawn_temp) "None" "SnapToTarget" "SnapToTarget" "KeepRelative" true)
  (`SceneComponent.SetVisibility` (`self.Blade`) false false))

(fn `UserConstructionScript`)