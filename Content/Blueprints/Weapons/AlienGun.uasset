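; Grabbable alien blaster that fires one LaserShot with a sound per index press and drains 10 energy from the player pawn.
; Pickup disables physics and snaps the handle to the given component, while Drop detaches it and restores physics; the holster attach is unwired.
; Custom depth serves as a highlight, updated each Tick from the pawn's right-hand target, which affects the targeted AlienGun rather than necessarily this one.
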(event `self.ReceiveBeginPlay`
  (`PrimitiveComponent.SetSimulatePhysics` (`self.Handle`) true))

(event `/Game/VirtualRealityBP/Blueprints/IndexInterface.IndexPressed`
  (bind (_returnvalue_location _returnvalue_rotation) (`KismetMathLibrary.BreakTransform` (`SceneComponent.K2_GetComponentToWorld` (`self.SpawnProjectile`))))
  (`/Engine/EditorBlueprintResources/StandardMacros.DoOnce` false :!label _label
    (:`Completed`
      (`|SpawnActorFromClass` "/Game/Blueprints/Weapons/Projectiles/LaserShot.LaserShot_C" (`KismetMathLibrary.MakeTransform` _returnvalue_location _returnvalue_rotation (1.0 1.0 1.0)) "Undefined" "OverrideRootScale")
      (`GameplayStatics.PlaySoundAtLocation` null _returnvalue_location)
      (message `/Game/Blueprints/Interfaces/EnergyInterface.DepleteEnergy` (`GameplayStatics.GetPlayerPawn` 0) 10.0))))

(event `/Game/VirtualRealityBP/Blueprints/IndexInterface.IndexReleased`
  (goto _label :!via `Reset`))

(event `/Game/VirtualRealityBP/Blueprints/PickupActorInterface.Pickup`
  (params (AttachTo :type "SceneComponent Object Reference"))
  (bind _handle (`self.Handle`))
  (`self.K2_DetachFromActor` "KeepWorld" "KeepWorld")
  (`PrimitiveComponent.SetSimulatePhysics` _handle false)
  (`SceneComponent.K2_AttachToComponent` _handle AttachTo "None" "SnapToTarget" "SnapToTarget" "KeepRelative" true)
  (`PrimitiveComponent.SetRenderCustomDepth` (`self.Blaster`) false))

(event `/Game/VirtualRealityBP/Blueprints/PickupActorInterface.Drop`
  (`PrimitiveComponent.SetSimulatePhysics` (`self.Handle`) true)
  (`self.K2_DetachFromActor` "KeepWorld" "KeepWorld")
  (`PrimitiveComponent.SetRenderCustomDepth` (`self.Blaster`) true)
  (bind _astwo_brothers_pawn_temp (cast `/Game/VirtualRealityBP/Blueprints/TwoBrothersPawnTEMP` (`GameplayStatics.GetPlayerPawn` 0))))

(event `self.ReceiveTick`
  (params (DeltaSeconds :type "Float (single-precision)"))
  (bind _astwo_brothers_pawn_temp (cast `/Game/VirtualRealityBP/Blueprints/TwoBrothersPawnTEMP` (`GameplayStatics.GetPlayerPawn` 0)))
  (bind _asalien_gun (cast `/Game/Blueprints/Weapons/AlienGun` (`/Game/VirtualRealityBP/Blueprints/TwoBrothersPawnTEMP.RightCurrentTargeted` _astwo_brothers_pawn_temp))
    (:`then`
      (`PrimitiveComponent.SetRenderCustomDepth` (`/Game/Blueprints/Weapons/AlienGun.Blaster` _asalien_gun) true))
    (:`CastFailed`
      (`PrimitiveComponent.SetRenderCustomDepth` (`self.Blaster`) false))))

(fn `UserConstructionScript`)