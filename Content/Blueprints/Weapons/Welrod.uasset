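; Welrod is a holdable pistol Blueprint that fires a bullet when its index input is pressed.
; A DoOnce gate spawns one scaled-down ClassicBullet at the SpawnProjectile transform per press and resets on release.
; Pickup turns off Handle physics and snaps it to the supplied component, while Drop restores physics and detaches the actor, keeping its world transform.
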(event `/Game/VirtualRealityBP/Blueprints/IndexInterface.IndexPressed`
  (bind (_returnvalue_location _returnvalue_rotation) (`KismetMathLibrary.BreakTransform` (`SceneComponent.K2_GetComponentToWorld` (`self.SpawnProjectile`))))
  (`/Engine/EditorBlueprintResources/StandardMacros.DoOnce` false :!label _label
    (:`Completed`
      (`|SpawnActorFromClass` "/Game/Blueprints/Weapons/ClassicBullet.ClassicBullet_C" (`KismetMathLibrary.MakeTransform` _returnvalue_location _returnvalue_rotation (0.03 0.03 0.03)) "Undefined" "OverrideRootScale"))))

(event `/Game/VirtualRealityBP/Blueprints/IndexInterface.IndexReleased`
  (goto _label :!via `Reset`))

(event `/Game/VirtualRealityBP/Blueprints/PickupActorInterface.Pickup`
  (params (AttachTo :type "SceneComponent Object Reference"))
  (bind _handle (`self.Handle`))
  (`PrimitiveComponent.SetSimulatePhysics` _handle false)
  (`SceneComponent.K2_AttachToComponent` _handle AttachTo "None" "SnapToTarget" "SnapToTarget" "KeepRelative" true))

(event `/Game/VirtualRealityBP/Blueprints/PickupActorInterface.Drop`
  (`PrimitiveComponent.SetSimulatePhysics` (`self.Handle`) true)
  (`self.K2_DetachFromActor` "KeepWorld" "KeepWorld"))

(fn `UserConstructionScript`)