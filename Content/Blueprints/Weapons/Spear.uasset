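; Spear weapon that can be picked up and dropped, serving as both a laser shooter and a contact weapon.
; Pickup disables physics on the Holder and snaps it to the given component; Drop re-enables physics and detaches.
; An index press fires one LaserShot with sound and drains player energy, gated by a DoOnce that resets on release.
; The Box overlap deals fixed damage to MovingTargetBP actors.
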(event `self.ReceiveBeginPlay`
  (`PrimitiveComponent.SetSimulatePhysics` (`self.Handle`) true))

(event `/Game/VirtualRealityBP/Blueprints/IndexInterface.IndexPressed`
  (bind (_returnvalue_location _returnvalue_rotation) (`KismetMathLibrary.BreakTransform` (`SceneComponent.K2_GetComponentToWorld` (`self.ProjectileSpawn`))))
  (`/Engine/EditorBlueprintResources/StandardMacros.DoOnce` false :!label _label
    (:`Completed`
      (`|SpawnActorFromClass` "/Game/Blueprints/Weapons/Projectiles/LaserShot.LaserShot_C" (`KismetMathLibrary.MakeTransform` _returnvalue_location _returnvalue_rotation (1.0 1.0 1.0)) "Undefined" "OverrideRootScale")
      (`GameplayStatics.PlaySoundAtLocation` "/Game/Audio/Sounds/Weapon_AssaultRifle/Stereo/AssaultRifle_Shot04_Stereo.AssaultRifle_Shot04_Stereo" _returnvalue_location)
      (message `/Game/Blueprints/Interfaces/EnergyInterface.DepleteEnergy` (`GameplayStatics.GetPlayerPawn` 0) 10.0))))

(event `/Game/VirtualRealityBP/Blueprints/IndexInterface.IndexReleased`
  (goto _label :!via `Reset`))

(event `/Game/VirtualRealityBP/Blueprints/PickupActorInterface.Pickup`
  (params (AttachTo :type "SceneComponent Object Reference"))
  (bind _holder (`self.Holder`))
  (`self.K2_DetachFromActor` "KeepWorld" "KeepWorld")
  (`PrimitiveComponent.SetSimulatePhysics` _holder false)
  (`SceneComponent.K2_AttachToComponent` _holder AttachTo "None" "SnapToTarget" "SnapToTarget" "KeepRelative" true))

(event `/Game/VirtualRealityBP/Blueprints/PickupActorInterface.Drop`
  (`PrimitiveComponent.SetSimulatePhysics` (`self.Holder`) true)
  (`self.K2_DetachFromActor` "KeepWorld" "KeepWorld"))

(event `self.Box.OnComponentBeginOverlap`
  (params (OverlappedComponent :type "PrimitiveComponent Object Reference") (OtherActor :type "Actor Object Reference") (OtherComp :type "PrimitiveComponent Object Reference") (OtherBodyIndex :type Integer) (bFromSweep :type Boolean) (SweepResult :type "HitResult Structure (by ref)"))
  (bind _asmoving_target_bp (cast `/Game/Blueprints/AI/BPMovingTarget/MovingTargetBP` OtherActor))
  (message `/Game/Blueprints/Interfaces/DamageInterface.DamageActor` _asmoving_target_bp 50.0))

(fn `UserConstructionScript`)