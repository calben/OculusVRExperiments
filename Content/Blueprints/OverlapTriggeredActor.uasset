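; Actor with three destructible parts, Left, Right and Head, that removes itself once all three are gone.
; OverlapBegin destroys whichever component is passed to it, then sets the matching destroyed flag if it is one of those parts.
; Tick polls the three flags every frame and destroys the actor when all are set.
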(event `self.ReceiveTick`
  (params (DeltaSeconds :type "Float (single-precision)"))
  (if (`self.LeftDestroyed`)
    (if (`self.RightDestroyed`)
      (if (`self.HeadDestroyed`)
        (`self.K2_DestroyActor`)))))

(event `/Game/VirtualRealityBP/Blueprints/OverlapTriggerInterface.OverlapBegin`
  (params (Instigator :type "ActorComponent Object Reference") (OverlapComponent :type "ActorComponent Object Reference"))
  (`ActorComponent.K2_DestroyComponent` OverlapComponent)
  (if (== OverlapComponent (`self.Left`))
    (set `self.LeftDestroyed` true)
    (elif (== OverlapComponent (`self.Right`))
      (set `self.RightDestroyed` true)
      (elif (== OverlapComponent (`self.Head`))
        (set `self.HeadDestroyed` true)))))

(fn `UserConstructionScript`)