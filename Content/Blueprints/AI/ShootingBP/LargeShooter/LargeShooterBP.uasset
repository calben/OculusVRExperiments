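; Large shooter enemy that patrols between its start point and an X-axis offset, and attacks the player on sight.
; A looping BrainTick timer checks range and line of sight, raising visible or lost events.
; When visible, it approaches, turns and fires two lasers; when lost, a do-once move targets the player's location.
; Tick drives randomly delayed patrols and, at zero health, enables mesh physics before delayed destruction.
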(event `self.ReceiveBeginPlay`
  (`KismetSystemLibrary.K2_SetTimer` null "BrainTick" 1.0 true)
  (set `self.Health` 50.0)
  (bind _output_get (set `self.StartLocation` (`SceneComponent.K2_GetComponentLocation` (`self.Box`))))
  (set `self.Point1` (+ _output_get (1000.0 0.0 0.0)))
  (set `CharacterMovementComponent.MaxWalkSpeed` (`self.MaxWalk`) (`self.CharacterMovement`))
  (`KismetSystemLibrary.Delay` 1.0)
  (`|AIMoveTo` self (`self.Point1`) null 5.0 true
    (:`then`
      (set `self.IsMoving` true))
    (:`OnSuccess`
      (set `self.AtStart` false)
      (set `self.IsMoving` false))
    (:`OnFail`
      (set `self.IsMoving` false))))

(event `self.ReceiveTick`
  (params (DeltaSeconds :type "Float (single-precision)"))
  (bind _returnvalue (`KismetMathLibrary.RandomFloatInRange` 0.0 4.0))
  (bind _mesh (`self.Mesh`))
  (`|ExecutionSequence`
    (:`then_0`
      (if (<= (`self.Health`) 0.0)
        (`PrimitiveComponent.SetSimulatePhysics` _mesh true)
        (`PrimitiveComponent.SetEnableGravity` _mesh true)
        (`KismetSystemLibrary.K2_PauseTimer` null "BrainTIck")
        (`KismetSystemLibrary.Delay` 20.0)
        (`self.K2_DestroyActor`)
        (elif (`self.PlayerVisible`)
          _
          (elif (`self.IsMoving`)
            _
            (elif (`self.AtStart`)
              (`KismetSystemLibrary.Delay` _returnvalue)
              (`|AIMoveTo` self (`self.Point1`) null 5.0 true
                (:`then`
                  (set `self.IsMoving` true))
                (:`OnSuccess`
                  (set `self.AtStart` false)
                  (set `self.IsMoving` false))
                (:`OnFail`
                  (set `self.IsMoving` false)))
              (else
                (`KismetSystemLibrary.Delay` _returnvalue)
                (`|AIMoveTo` self (`self.StartLocation`) null 5.0 true
                  (:`then`
                    (set `self.IsMoving` true))
                  (:`OnSuccess`
                    (set `self.AtStart` true)
                    (set `self.IsMoving` false))
                  (:`OnFail`
                    (set `self.IsMoving` false)))))))))))

(event `EnemyBecameVisible`
  (bind (_returnvalue_location _returnvalue_rotation) (`KismetMathLibrary.BreakTransform` (`SceneComponent.K2_GetComponentToWorld` (`self.ProjectileSpawn`))))
  (bind (_returnvalue_location_2 _returnvalue_rotation_2) (`KismetMathLibrary.BreakTransform` (`SceneComponent.K2_GetComponentToWorld` (`self.ProjectileSpawn2`))))
  (bind (_returnvalue_roll _returnvalue_pitch _returnvalue_yaw) (`KismetMathLibrary.BreakRotator` (`KismetMathLibrary.FindLookAtRotation` (`SceneComponent.K2_GetComponentLocation` (`self.Box`)) (`self.K2_GetActorLocation` (`GameplayStatics.GetPlayerPawn` 0)))))
  (set `self.AtStart` false)
  (`|AIMoveTo` self (0.0 0.0 0.0) (`GameplayStatics.GetPlayerPawn` 0) 1000.0 true
    (:`then`
      (set `self.IsMoving` true))
    (:`OnSuccess`
      (set `self.IsMoving` false)
      (`self.K2_SetActorRotation` (`KismetMathLibrary.MakeRotator` _returnvalue_roll 0.0 _returnvalue_yaw))
      (`|SpawnActorFromClass` "/Game/Blueprints/Weapons/Projectiles/LaserShot.LaserShot_C" (`KismetMathLibrary.MakeTransform` _returnvalue_location _returnvalue_rotation (0.5 0.5 0.5)) "Undefined" "OverrideRootScale")
      (`GameplayStatics.PlaySoundAtLocation` "/Game/Audio/Sounds/Weapon_AssaultRifle/Stereo/AssaultRifle_ShotEnd04_Stereo.AssaultRifle_ShotEnd04_Stereo" _returnvalue_location)
      (`|SpawnActorFromClass` "/Game/Blueprints/Weapons/Projectiles/LaserShot.LaserShot_C" (`KismetMathLibrary.MakeTransform` _returnvalue_location_2 _returnvalue_rotation_2 (0.5 0.5 0.5)) "Undefined" "OverrideRootScale")
      (`GameplayStatics.PlaySoundAtLocation` "/Game/Audio/Sounds/Weapon_AssaultRifle/Stereo/AssaultRifle_ShotEnd04_Stereo.AssaultRifle_ShotEnd04_Stereo" _returnvalue_location))))

(event `EnemyLost`
  (`|DoOnceMultiInput`
    (:`A Out`
      (bind _output_get (set `self.PlayerLostLocation` (`self.K2_GetActorLocation` (`GameplayStatics.GetPlayerPawn` 0))))
      (`|AIMoveTo` self _output_get))))

(event `/Game/Blueprints/Interfaces/DamageInterface.DamageActor`
  (params (DamageAmount :type "Float (single-precision)"))
  (set `self.Health` (- (`self.Health`) DamageAmount)))

(fn `BrainTick`
  (bind _returnvalue (`SceneComponent.K2_GetComponentLocation` (`self.Box`)))
  (bind _returnvalue_2 (`self.K2_GetActorLocation` (`GameplayStatics.GetPlayerPawn` 0)))
  (bind _outactors (`GameplayStatics.GetAllActorsOfClass` "/Game/VirtualRealityBP/Blueprints/TwoBrothersPawnTEMP.TwoBrothersPawnTEMP_C"))
  (if (<= (`KismetMathLibrary.VSize` (- _returnvalue _returnvalue_2)) 3000.0)
    (bind (_outhit _returnvalue_3) (`KismetSystemLibrary.LineTraceSingle` _returnvalue _returnvalue_2 "TraceTypeQuery2" false _outactors "ForOneFrame"))
    (if _returnvalue_3
      (set `self.PlayerVisible` false)
      (`self.EnemyLost`)
      (elif (not (`self.MeleeEnabled`))
        (set `self.PlayerVisible` true)
        (`self.EnemyBecameVisible`)))))

(fn `UserConstructionScript`)