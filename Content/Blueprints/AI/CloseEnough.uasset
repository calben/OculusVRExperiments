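; CloseEnough is a behavior tree decorator that checks whether a follower AI is close enough to the actor it follows.
; It casts the owner to FollowerAICon, caches that controller and reads the TargetToFollow actor from the blackboard.
; The condition passes when the distance between that actor and the controlled pawn is within AcceptableDistance.
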(fn `PerformConditionCheck`
  (params (OwnerActor :type "Actor Object Reference"))
  (returns (ReturnValue :type Boolean))
  (bind _asfollower_aicon (cast `/Game/Blueprints/AI/FollowerAICon` OwnerActor)
    (:`then`
      (set `self.AIConRef` _asfollower_aicon))
    (:`CastFailed`
      _))
  (return (<= (`KismetMathLibrary.VSize` (- (`Actor.K2_GetActorLocation` (`BTFunctionLibrary.GetBlackboardValueAsActor` (`self.Target to Follow`))) (`Actor.K2_GetActorLocation` (`Controller.K2_GetPawn` (`self.AIConRef`))))) (`self.AcceptableDistance`))))