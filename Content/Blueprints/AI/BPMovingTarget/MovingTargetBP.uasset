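; Parasite enemy AI that patrols between its spawn point and an offset point, chases the visible player, and dies when health runs out.
; A looping BrainTick timer line-traces to nearby players, triggering an AIMoveTo chase or a one-shot move to the player's position when sight is blocked.
; Reaching the player sets MeleeEnabled, pausing re-chase until Tick sees them move away.
; Hand collision overlaps damage TwoBrothersPawnTEMP, with sounds for breathing and attacks.
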(event `self.ReceiveBeginPlay`
  (`KismetSystemLibrary.K2_SetTimer` null "BrainTick" 2.0 true)
  (set `self.Health` 50.0)
  (bind _output_get (set `self.StartLocation` (`SceneComponent.K2_GetComponentLocation` (`self.Mesh`))))
  (set `self.Point1` (+ _output_get (0.0 500.0 0.0)))
  (set `CharacterMovementComponent.MaxWalkSpeed` (`self.MaxWalk`) (`self.CharacterMovement`))
  (`KismetSystemLibrary.Delay` 1.0)
  (`|AIMoveTo` self (`self.Point1`) null 5.0 true
    (:`then`
      (set `self.IsMoving` true))
    (:`OnSuccess`
      (set `self.AtStart` false)
      (set `self.IsMoving` false))
    (:`OnFail`
      (set `self.IsMoving` false))))

(event `self.ReceiveTick`
  (params (DeltaSeconds :type "Float (single-precision)"))
  (bind _returnvalue (`KismetMathLibrary.RandomFloatInRange` 0.0 4.0))
  (bind _head (`self.Head`))
  (`|ExecutionSequence`
    (:`then_0`
      (if (<= (`self.Health`) 0.0)
        (`self.K2_DestroyActor`)
        (elif (`self.PlayerVisible`)
          _
          (elif (`self.IsMoving`)
            (goto _label :!via `Reset`)
            (elif (`self.AtStart`)
              (`KismetSystemLibrary.Delay` _returnvalue)
              (`|AIMoveTo` self (`self.Point1`) null 5.0 true
                (:`then`
                  (set `self.IsMoving` true)
                  (`AudioComponent.Play` (`self.Breathing`) 0.0))
                (:`OnSuccess`
                  (set `self.AtStart` false)
                  (set `self.IsMoving` false))
                (:`OnFail`
                  (set `self.IsMoving` false)))
              (else
                (`KismetSystemLibrary.Delay` _returnvalue)
                (`|AIMoveTo` self (`self.StartLocation`) null 5.0 true
                  (:`then`
                    (set `self.IsMoving` true)
                    (`AudioComponent.Play` (`self.Breathing`) 0.0))
                  (:`OnSuccess`
                    (set `self.AtStart` true)
                    (set `self.IsMoving` false))
                  (:`OnFail`
                    (set `self.IsMoving` false)))))))))
    (:`then_1`
      (if (`self.MeleeEnabled`)
        (if (>= (`KismetMathLibrary.VSize` (- (`SceneComponent.K2_GetComponentLocation` (`self.Head`)) (`self.K2_GetActorLocation` (`GameplayStatics.GetPlayerPawn` 0)))) 300.0)
          (set `self.MeleeEnabled` false))))))

(event `EnemyBecameVisible`
  (bind _head (`self.Head`))
  (set `self.AtStart` false)
  (`|AIMoveTo` self (0.0 0.0 0.0) (`GameplayStatics.GetPlayerPawn` 0) 50.0 true
    (:`then`
      (set `self.IsMoving` true)
      (`/Engine/EditorBlueprintResources/StandardMacros.DoOnce` false :!label _label
        (:`Completed`
          (bind _returnvalue (`GameplayStatics.SpawnSoundAttached` "/Game/Audio/Parasite/ParasiteBreathing.ParasiteBreathing" _head "None" (0.0 0.0 0.0) (struct) "SnapToTarget" true 10.0))
          (bind _output_get (set `self.BreathingCue` _returnvalue))
          (`AudioComponent.Play` _output_get 0.0)
          (`GameplayStatics.PlaySoundAtLocation` "/Game/Audio/Parasite/ParasiteEnemySeen.ParasiteEnemySeen" (`SceneComponent.K2_GetComponentLocation` _head)))))
    (:`OnSuccess`
      (set `self.IsMoving` false)
      (set `self.MeleeEnabled` true)
      (`GameplayStatics.PlaySoundAtLocation` "/Game/Audio/Parasite/ParasitePunch.ParasitePunch" (`SceneComponent.K2_GetComponentLocation` (`self.Head`)))
      (goto _label_2 :!via `Reset In`))))

(event `EnemyLost`
  (`|DoOnceMultiInput` :!label _label_2
    (:`A Out`
      (bind _output_get (set `self.PlayerLostLocation` (`self.K2_GetActorLocation` (`GameplayStatics.GetPlayerPawn` 0))))
      (`|AIMoveTo` self _output_get))))

(event `/Game/Blueprints/Interfaces/DamageInterface.DamageActor`
  (params (DamageAmount :type "Float (single-precision)"))
  (set `self.Health` (- (`self.Health`) DamageAmount)))

(event `self.LeftHandCollision.OnComponentBeginOverlap`
  (params (OverlappedComponent :type "PrimitiveComponent Object Reference") (OtherActor :type "Actor Object Reference") (OtherComp :type "PrimitiveComponent Object Reference") (OtherBodyIndex :type Integer) (bFromSweep :type Boolean) (SweepResult :type "HitResult Structure (by ref)"))
  (bind _astwo_brothers_pawn_temp (cast `/Game/VirtualRealityBP/Blueprints/TwoBrothersPawnTEMP` OtherActor))
  (message `/Game/Blueprints/Interfaces/DamageInterface.DamageActor` _astwo_brothers_pawn_temp 20.0))

(event `self.RightHandCollision.OnComponentBeginOverlap`
  (params (OverlappedComponent :type "PrimitiveComponent Object Reference") (OtherActor :type "Actor Object Reference") (OtherComp :type "PrimitiveComponent Object Reference") (OtherBodyIndex :type Integer) (bFromSweep :type Boolean) (SweepResult :type "HitResult Structure (by ref)"))
  (bind _astwo_brothers_pawn_temp (cast `/Game/VirtualRealityBP/Blueprints/TwoBrothersPawnTEMP` OtherActor))
  (message `/Game/Blueprints/Interfaces/DamageInterface.DamageActor` _astwo_brothers_pawn_temp 20.0)
  (`GameplayStatics.PlaySoundAtLocation` null (`SceneComponent.K2_GetComponentLocation` (`self.RightHandCollision`))))

(fn `BrainTick`
  (bind _returnvalue (`SceneComponent.K2_GetComponentLocation` (`self.Head`)))
  (bind _returnvalue_2 (`self.K2_GetActorLocation` (`GameplayStatics.GetPlayerPawn` 0)))
  (bind _outactors (`GameplayStatics.GetAllActorsOfClass` "/Game/VirtualRealityBP/Blueprints/TwoBrothersPawnTEMP.TwoBrothersPawnTEMP_C"))
  (if (<= (`KismetMathLibrary.VSize` (- _returnvalue _returnvalue_2)) 3000.0)
    (bind (_outhit _returnvalue_3) (`KismetSystemLibrary.LineTraceSingle` _returnvalue _returnvalue_2 "TraceTypeQuery2" false _outactors "ForOneFrame"))
    (if _returnvalue_3
      (set `self.PlayerVisible` false)
      (`self.EnemyLost`)
      (elif (not (`self.MeleeEnabled`))
        (set `self.PlayerVisible` true)
        (`self.EnemyBecameVisible`)))))

(fn `UserConstructionScript`)