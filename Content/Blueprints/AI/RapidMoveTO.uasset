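; Behavior tree task for follower AI that moves the controlled pawn toward the actor stored in the TargetToFollow blackboard key.
; On execute it caches the owner as a FollowerAICon if not already set, then runs AIMoveTo with a small fixed acceptance radius.
; A successful move finishes the task as failed, and a failed move has no handler to finish it.
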(event `self.ReceiveExecute`
  (params (OwnerActor :type "Actor Object Reference"))
  (if (not (!= (`self.AI CON Ref`) null))
    (bind _asfollower_aicon (cast `/Game/Blueprints/AI/FollowerAICon` OwnerActor))
    (set `self.AI CON Ref` _asfollower_aicon))
  (`|AIMoveTo` (`Controller.K2_GetPawn` (`self.AI CON Ref`)) (0.0 0.0 0.0) (`BTFunctionLibrary.GetBlackboardValueAsActor` (`self.Target to Follow`)) 50.0
    (:`OnSuccess`
      (`self.FinishExecute` false))))