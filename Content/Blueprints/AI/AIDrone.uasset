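; AI drone actor with a health pool that explodes when destroyed.
; BeginPlay fills health from MaxHealth, the DamageActor event subtracts from it, and Tick checks for it reaching zero.
; Overlap of DroneHitBox with the player pawn's HeadCollision triggers the same death path regardless of health.
; Death spawns a ProjectileImpactBlast at the hit box transform and destroys the drone.
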(event `self.ReceiveBeginPlay`
  (set `self.CurrentHealth` (`self.MaxHealth`)))

(event `self.ReceiveTick`
  (params (DeltaSeconds :type "Float (single-precision)"))
  (if (<= (`self.CurrentHealth`) 0.0)
    (`|SpawnActorFromClass` "/Game/Blueprints/ProjectileImpactBlast.ProjectileImpactBlast_C" (`SceneComponent.K2_GetComponentToWorld` (`self.DroneHitBox`)) "Undefined" "OverrideRootScale" :!label _label)
    (`self.K2_DestroyActor`)))

(event `self.DroneHitBox.OnComponentBeginOverlap`
  (params (OverlappedComponent :type "PrimitiveComponent Object Reference") (OtherActor :type "Actor Object Reference") (OtherComp :type "PrimitiveComponent Object Reference") (OtherBodyIndex :type Integer) (bFromSweep :type Boolean) (SweepResult :type "HitResult Structure (by ref)"))
  (bind _astwo_brothers_pawn_temp (cast `/Game/VirtualRealityBP/Blueprints/TwoBrothersPawnTEMP` (`GameplayStatics.GetPlayerPawn` 0)))
  (if (!= OtherActor self)
    (if (== OtherComp (`/Game/VirtualRealityBP/Blueprints/TwoBrothersPawnTEMP.HeadCollision` _astwo_brothers_pawn_temp))
      (goto _label))))

(event `/Game/Blueprints/DamageInterface.DamageActor`
  (params (DamageAmount :type "Float (single-precision)"))
  (set `self.CurrentHealth` (- (`self.CurrentHealth`) DamageAmount)))

(fn `UserConstructionScript`)