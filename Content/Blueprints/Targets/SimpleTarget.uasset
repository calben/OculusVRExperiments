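; SimpleTarget is a shootable target actor that tracks health and a hit count, starting at full health on BeginPlay.
; A LaserShot hitting the CylinderFace component, or a call to the DamageActor event, subtracts a fixed amount of health and increments the hit count.
; Tick polls health and, once it is depleted, plays a rifle shot sound at the face's location and destroys the actor.
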(event `self.ReceiveBeginPlay`
  (set `self.Health` 100.0)
  (set `self.HitNumber` 0))

(event `self.ReceiveTick`
  (params (DeltaSeconds :type "Float (single-precision)"))
  (if (<= (`self.Health`) 0.0)
    (`GameplayStatics.PlaySoundAtLocation` "/Game/Assets/Audio/Sounds/Weapon_AssaultRifle/Stereo/AssaultRifle_Shot04_Stereo.AssaultRifle_Shot04_Stereo" (`SceneComponent.K2_GetComponentLocation` (`self.CylinderFace`)))
    (`self.K2_DestroyActor`)))

(event `self.CylinderFace.OnComponentHit`
  (params (HitComponent :type "PrimitiveComponent Object Reference") (OtherActor :type "Actor Object Reference") (OtherComp :type "PrimitiveComponent Object Reference") (NormalImpulse :type "Vector Structure") (Hit :type "HitResult Structure (by ref)"))
  (cast `/Game/Blueprints/Weapons/Projectiles/LaserShot` OtherActor)
  (set `self.Health` (- (`self.Health`) 10.0) :!label _label)
  (set `self.HitNumber` (+ (`self.HitNumber`) 1)))

(event `/Game/Blueprints/Interfaces/DamageInterface.DamageActor`
  (params (DamageAmount :type "Float (single-precision)"))
  (goto _label))

(fn `UserConstructionScript`)