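; Hammer tool actor that can be picked up and dropped, and damages moving targets it hits.
; Pickup turns off physics on the Handle and snaps it to the supplied component.
; Drop re-enables physics and detaches, then after a short delay snaps the Handle back to the player pawn's Holster1.
; Any HammerHead overlap with a MovingTargetBP sends it fixed damage through DamageActorMessage.
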(event `/Game/VirtualRealityBP/Blueprints/PickupActorInterface.Pickup`
  (params (AttachTo :type "SceneComponent Object Reference"))
  (bind _handle (`self.Handle`))
  (`self.K2_DetachFromActor` "KeepWorld" "KeepWorld")
  (`PrimitiveComponent.SetSimulatePhysics` _handle false)
  (`SceneComponent.K2_AttachToComponent` _handle AttachTo "None" "SnapToTarget" "SnapToTarget" "KeepRelative" true))

(event `/Game/VirtualRealityBP/Blueprints/PickupActorInterface.Drop`
  (`PrimitiveComponent.SetSimulatePhysics` (`self.Handle`) true)
  (`self.K2_DetachFromActor` "KeepWorld" "KeepWorld")
  (`KismetSystemLibrary.Delay` 4.0)
  (bind _astwo_brothers_pawn_temp (cast `/Game/VirtualRealityBP/Blueprints/TwoBrothersPawnTEMP` (`GameplayStatics.GetPlayerPawn` 0)))
  (`SceneComponent.K2_AttachToComponent` (`self.Handle`) (`/Game/VirtualRealityBP/Blueprints/TwoBrothersPawnTEMP.Holster1` _astwo_brothers_pawn_temp) "None" "SnapToTarget" "SnapToTarget" "KeepRelative" true))

(event `self.HammerHead.OnComponentBeginOverlap`
  (params (OverlappedComponent :type "PrimitiveComponent Object Reference") (OtherActor :type "Actor Object Reference") (OtherComp :type "PrimitiveComponent Object Reference") (OtherBodyIndex :type Integer) (bFromSweep :type Boolean) (SweepResult :type "HitResult Structure (by ref)"))
  (bind _asmoving_target_bp (cast `/Game/Blueprints/AI/BPMovingTarget/MovingTargetBP` OtherActor))
  (message `/Game/Blueprints/Interfaces/DamageInterface.DamageActor` _asmoving_target_bp 20.0))

(fn `UserConstructionScript`)