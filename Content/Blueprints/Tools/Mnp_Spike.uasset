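; Grabbable spike prop that damages MiniParasite and LargeShooterBP enemies when its mesh hits them.
; Pickup turns off physics and attaches it to the given component, while Drop detaches it and restores physics.
; Each tick it reads the player pawn's right-hand target, enabling custom depth on a targeted BP_PickupCube or otherwise disabling it on its own mesh.
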(event `/Game/VirtualRealityBP/Blueprints/PickupActorInterface.Pickup`
  (params (AttachTo :type "SceneComponent Object Reference"))
  (`PrimitiveComponent.SetSimulatePhysics` (`self.StaticMeshComponent`) false)
  (`SceneComponent.K2_AttachToComponent` (`self.K2_GetRootComponent`) AttachTo "None" "KeepWorld" "KeepWorld" "KeepWorld" false))

(event `/Game/VirtualRealityBP/Blueprints/PickupActorInterface.Drop`
  (`PrimitiveComponent.SetSimulatePhysics` (`self.StaticMeshComponent`) true)
  (`self.K2_DetachFromActor` "KeepWorld" "KeepWorld" "KeepWorld"))

(event `self.ReceiveTick`
  (params (DeltaSeconds :type "Float (single-precision)"))
  (bind _astwo_brothers_pawn_temp (cast `/Game/VirtualRealityBP/Blueprints/TwoBrothersPawnTEMP` (`GameplayStatics.GetPlayerPawn` 0)))
  (bind _asbp_pickup_cube (cast `/Game/VirtualRealityBP/Blueprints/BP_PickupCube` (`/Game/VirtualRealityBP/Blueprints/TwoBrothersPawnTEMP.RightCurrentTargeted` _astwo_brothers_pawn_temp))
    (:`then`
      (`PrimitiveComponent.SetRenderCustomDepth` (`StaticMeshActor.StaticMeshComponent` _asbp_pickup_cube) true))
    (:`CastFailed`
      (`PrimitiveComponent.SetRenderCustomDepth` (`self.StaticMeshComponent`) false))))

(event `self.StaticMeshComponent.OnComponentHit`
  (params (HitComponent :type "PrimitiveComponent Object Reference") (OtherActor :type "Actor Object Reference") (OtherComp :type "PrimitiveComponent Object Reference") (NormalImpulse :type "Vector Structure") (Hit :type "HitResult Structure (by ref)"))
  (cast `/Game/Blueprints/AI/BP_MiniParasite/MiniParasite` OtherActor
    (:`then`
      _)
    (:`CastFailed`
      (cast `/Game/Blueprints/AI/ShootingBP/LargeShooter/LargeShooterBP` OtherActor)))
  (message `/Game/Blueprints/Interfaces/DamageInterface.DamageActor` OtherActor 100.0))

(fn `UserConstructionScript`)