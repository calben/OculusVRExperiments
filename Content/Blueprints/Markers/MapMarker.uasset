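; Map marker actor that runs a Simon Says memory test on four overlap-triggered pads, hidden at start.
; Tick replays the random sequence on game-time offsets, then opens input, ending at four steps.
; Overlaps light pads via material swaps with timed dimming by TestingMode, and check input, extending the sequence after each completed round.
; BeginSession and Reset are empty, and the timer-called BeginDisplay is absent, so nothing here starts playback.
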(event `self.ReceiveBeginPlay`
  (bind _2 (`self.2`))
  (bind _4 (`self.4`))
  (bind _3 (`self.3`))
  (bind _1 (`self.1`))
  (`PrimitiveComponent.SetMaterial` _1 0 "/Game/Assets/Mesh/Utils/Materials/MemoryPawnDefault.MemoryPawnDefault")
  (`SceneComponent.SetVisibility` _1 false false)
  (`PrimitiveComponent.SetMaterial` _2 0 "/Game/Assets/Mesh/Utils/Materials/MemoryPawnDefault.MemoryPawnDefault")
  (`SceneComponent.SetVisibility` _2 false false)
  (`PrimitiveComponent.SetMaterial` _3 0 "/Game/Assets/Mesh/Utils/Materials/MemoryPawnDefault.MemoryPawnDefault")
  (`SceneComponent.SetVisibility` _3 false false)
  (`PrimitiveComponent.SetMaterial` _4 0 "/Game/Assets/Mesh/Utils/Materials/MemoryPawnDefault.MemoryPawnDefault")
  (`SceneComponent.SetVisibility` _4 false false)
  (set `self.AcceptingInput` false)
  (set `self.DisplayingSequence` false))

(event `/Game/VirtualRealityBP/Blueprints/OverlapTriggerInterface.OverlapBegin`
  (params (Instigator :type "ActorComponent Object Reference") (OverlapComponent :type "ActorComponent Object Reference"))
  (if (== OverlapComponent null)
    (`self.BeginSession`)
    (elif (== OverlapComponent (`self.1`))
      (`self.LightUp` 1)
      (`self.TestInput` 1)
      (elif (== OverlapComponent (`self.2`))
        (`self.LightUp` 2)
        (`self.TestInput` 2)
        (elif (== OverlapComponent (`self.3`))
          (`self.LightUp` 3)
          (`self.TestInput` 3)
          (elif (== OverlapComponent (`self.4`))
            (`self.LightUp` 4)
            (`self.TestInput` 4)))))))

(event `self.ReceiveTick`
  (params (DeltaSeconds :type "Float (single-precision)"))
  (bind _item (`KismetArrayLibrary.Array_Get` (`self.SimonSaysSequence`) (`self.DisplayIndex`)))
  (bind _returnvalue (`KismetArrayLibrary.Array_Length` (`self.SimonSaysSequence`)))
  (if (`self.DisplayingSequence`)
    (if (>= _returnvalue 4)
      (`/Engine/EditorBlueprintResources/StandardMacros.DoOnce` false
        (:`Completed`
          (set `self.Testing` false)
          (set `self.DisplayIndex` 0)
          (set `self.TestIndex` 0)
          (set `self.DisplayingSequence` false)
          (`SceneComponent.SetVisibility` (`self.1`) false false)
          (`SceneComponent.SetVisibility` (`self.2`) false false)
          (`SceneComponent.SetVisibility` (`self.3`) false false)
          (`SceneComponent.SetVisibility` (`self.4`) false false)))
      (elif (< (`self.DisplayIndex`) _returnvalue)
        (if (`KismetMathLibrary.NearlyEqual_FloatFloat` (- (`KismetSystemLibrary.GetGameTimeInSeconds`) (`self.DisplayStartTime`)) (/ (`KismetMathLibrary.Conv_IntToDouble` (`self.DisplayIndex`)) 1.0) 0.1)
          (`/Engine/EditorBlueprintResources/StandardMacros.DoOnce` false :!label _label
            (:`Completed`
              (`KismetSystemLibrary.PrintString` "Checkpoint")
              (if (== _item 1)
                (`self.LightUp` 1)
                (set `self.DisplayIndex` (+ (`self.DisplayIndex`) 1))
                (elif (== _item 2)
                  (`self.LightUp` 2)
                  (set `self.DisplayIndex` (+ (`self.DisplayIndex`) 1))
                  (elif (== _item 3)
                    (`self.LightUp` 3)
                    (set `self.DisplayIndex` (+ (`self.DisplayIndex`) 1))
                    (elif (== _item 4)
                      (`self.LightUp` 4)
                      (set `self.DisplayIndex` (+ (`self.DisplayIndex`) 1))))))))
          (elif (>= (- (`KismetSystemLibrary.GetGameTimeInSeconds`) (`self.DisplayStartTime`)) (+ (`KismetMathLibrary.Conv_IntToDouble` (/ _returnvalue 2)) 2.0))
            (set `self.DisplayingSequence` false)
            (set `self.AcceptingInput` true)
            (set `self.TestIndex` 0)
            (set `self.DisplayIndex` 0)
            (goto _label :!via `Reset`)
            (else
              (goto _label :!via `Reset`))))
        (else
          (set `self.DisplayingSequence` false)
          (set `self.AcceptingInput` true)
          (set `self.TestIndex` 0)
          (set `self.DisplayIndex` 0)
          (goto _label :!via `Reset`))))))

(fn `BeginSession`)

(fn `Dim1`
  (bind _testingmode (`self.TestingMode`))
  (if (`|EnumEquality` _testingmode "NewEnumerator0")
    (`PrimitiveComponent.SetMaterial` (`self.1`) 0 "/Game/Assets/Mesh/Utils/Materials/MemoryPawnDefault.MemoryPawnDefault")
    (elif (`|EnumEquality` _testingmode "NewEnumerator1")
      (`PrimitiveComponent.SetMaterial` (`self.1`) 0 "/Game/Assets/Mesh/Utils/Materials/SimonSays1.SimonSays1"))))

(fn `Dim2`
  (bind _testingmode (`self.TestingMode`))
  (bind _2 (`self.2`))
  (if (`|EnumEquality` _testingmode "NewEnumerator0")
    (`PrimitiveComponent.SetMaterial` _2 0 "/Game/Assets/Mesh/Utils/Materials/MemoryPawnDefault.MemoryPawnDefault")
    (elif (`|EnumEquality` _testingmode "NewEnumerator1")
      (`PrimitiveComponent.SetMaterial` _2 0 "/Game/Assets/Mesh/Utils/Materials/SimonSays2.SimonSays2"))))

(fn `Dim3`
  (bind _testingmode (`self.TestingMode`))
  (bind _3 (`self.3`))
  (if (`|EnumEquality` _testingmode "NewEnumerator0")
    (`PrimitiveComponent.SetMaterial` _3 0 "/Game/Assets/Mesh/Utils/Materials/MemoryPawnDefault.MemoryPawnDefault")
    (elif (`|EnumEquality` _testingmode "NewEnumerator1")
      (`PrimitiveComponent.SetMaterial` _3 0 "/Game/Assets/Mesh/Utils/Materials/SimonSays3.SimonSays3"))))

(fn `Dim4`
  (bind _testingmode (`self.TestingMode`))
  (bind _4 (`self.4`))
  (if (`|EnumEquality` _testingmode "NewEnumerator0")
    (`PrimitiveComponent.SetMaterial` _4 0 "/Game/Assets/Mesh/Utils/Materials/MemoryPawnDefault.MemoryPawnDefault")
    (elif (`|EnumEquality` _testingmode "NewEnumerator1")
      (`PrimitiveComponent.SetMaterial` _4 0 "/Game/Assets/Mesh/Utils/Materials/SimonSays4.SimonSays4"))))

(fn `DimAll`
  (`self.Dim1`)
  (`self.Dim2`)
  (`self.Dim3`)
  (`self.Dim4`))

(fn `Light1`
  (`PrimitiveComponent.SetMaterial` (`self.1`) 0 "/Game/Assets/Mesh/Utils/Materials/SimonSays1lit.SimonSays1lit")
  (`KismetSystemLibrary.K2_SetTimer` null "Dim1" (`self.StimulusDelay`)))

(fn `Light2`
  (`PrimitiveComponent.SetMaterial` (`self.2`) 0 "/Game/Assets/Mesh/Utils/Materials/SimonSays2lit.SimonSays2lit")
  (`KismetSystemLibrary.K2_SetTimer` null "Dim2" (`self.StimulusDelay`)))

(fn `Light3`
  (`PrimitiveComponent.SetMaterial` (`self.3`) 0 "/Game/Assets/Mesh/Utils/Materials/SimonSays3lit.SimonSays3lit")
  (`KismetSystemLibrary.K2_SetTimer` null "Dim3" (`self.StimulusDelay`)))

(fn `Light4`
  (`PrimitiveComponent.SetMaterial` (`self.4`) 0 "/Game/Assets/Mesh/Utils/Materials/SimonSays4lit.SimonSays4lit")
  (`KismetSystemLibrary.K2_SetTimer` null "Dim4" (`self.StimulusDelay`)))

(fn `LightAll`
  (`self.LightUp` 1)
  (`self.LightUp` 2)
  (`self.LightUp` 3)
  (`self.LightUp` 4))

(fn `LightUp`
  (params (Light :type Integer))
  (if (== Light 1)
    (`PrimitiveComponent.SetMaterial` (`self.1`) 0 "/Game/Assets/Mesh/Utils/Materials/SimonSays1lit.SimonSays1lit")
    (`KismetSystemLibrary.K2_SetTimer` null "Dim1" (`self.StimulusDelay`))
    (elif (== Light 2)
      (`PrimitiveComponent.SetMaterial` (`self.2`) 0 "/Game/Assets/Mesh/Utils/Materials/SimonSays2lit.SimonSays2lit")
      (`KismetSystemLibrary.K2_SetTimer` null "Dim2" (`self.StimulusDelay`))
      (elif (== Light 3)
        (`PrimitiveComponent.SetMaterial` (`self.3`) 0 "/Game/Assets/Mesh/Utils/Materials/SimonSays3lit.SimonSays3lit")
        (`KismetSystemLibrary.K2_SetTimer` null "Dim3" (`self.StimulusDelay`))
        (elif (== Light 4)
          (`PrimitiveComponent.SetMaterial` (`self.4`) 0 "/Game/Assets/Mesh/Utils/Materials/SimonSays4lit.SimonSays4lit")
          (`KismetSystemLibrary.K2_SetTimer` null "Dim4" (`self.StimulusDelay`)))))))

(fn `Reset`)

(fn `TestInput`
  (params (InputNumber :type Integer))
  (if (`self.AcceptingInput`)
    (if (== InputNumber (`KismetArrayLibrary.Array_Get` (`self.SimonSaysSequence`) (`self.TestIndex`)))
      (`KismetSystemLibrary.PrintString` "Correct")
      (bind _output_get (set `self.TestIndex` (+ (`self.TestIndex`) 1)))
      (if (>= _output_get (`KismetArrayLibrary.Array_Length` (`self.SimonSaysSequence`)))
        (`KismetSystemLibrary.PrintString` "Extending ")
        (set `self.AcceptingInput` false)
        (`KismetArrayLibrary.Array_Append` (`self.SimonSaysSequence`) (`|MakeArray` (`KismetMathLibrary.RandomIntegerInRange` 1 4)))
        (`KismetSystemLibrary.K2_SetTimer` null "BeginDisplay" 1.0))
      (else
        (`KismetSystemLibrary.PrintString` "Incorrect")
        (`self.Reset`)))))

(fn `UpdateDisplay`)

(fn `UserConstructionScript`)