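; TargetBlock is a damageable actor that is destroyed when its health runs out.
; BeginPlay sets CurrentHealth to MaxHealth, and the custom DamageActor event subtracts the incoming amount and prints the remaining health as debug output.
; Tick polls health every frame and destroys the actor at zero or below, so the death check is separate from the damage event.
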(event `self.ReceiveBeginPlay`
  (set `self.CurrentHealth` (`self.MaxHealth`)))

(event `/Game/Assets/BP/DamageInterface.DamageActor`
  (params (DamageAmount :type "Float (single-precision)"))
  (bind _output_get (set `self.CurrentHealth` (- (`self.CurrentHealth`) DamageAmount)))
  (`KismetSystemLibrary.PrintString` (`KismetStringLibrary.Conv_DoubleToString` _output_get)))

(event `self.ReceiveTick`
  (params (DeltaSeconds :type "Float (single-precision)"))
  (if (<= (`self.CurrentHealth`) 0.0)
    (`self.K2_DestroyActor`)))

(fn `UserConstructionScript`)