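; DodgeWall is a wall Blueprint with a right-hand target component that registers a hit from the player.
; When HandRIght overlaps the player pawn and the wall's owner casts to TwoBrothersPawnTEMP, it destroys that component and sets HandRightHit.
; A check against the right controller's GrabSphere is left unconnected, and Tick has an empty branch.
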(event `self.ReceiveTick`
  (params (DeltaSeconds :type "Float (single-precision)"))
  (if true
    _))

(event `self.HandRIght.OnComponentBeginOverlap`
  (params (OverlappedComponent :type "PrimitiveComponent Object Reference") (OtherActor :type "Actor Object Reference") (OtherComp :type "PrimitiveComponent Object Reference") (OtherBodyIndex :type Integer) (bFromSweep :type Boolean) (SweepResult :type "HitResult Structure (by ref)"))
  (if (== OtherActor (`GameplayStatics.GetPlayerPawn` 0))
    (bind _astwo_brothers_pawn_temp (cast `/Game/VirtualRealityBP/Blueprints/TwoBrothersPawnTEMP` (`self.GetOwner`)))
    (`ActorComponent.K2_DestroyComponent` (`self.HandRIght`))
    (set `self.HandRightHit` true)))

(fn `UserConstructionScript`)