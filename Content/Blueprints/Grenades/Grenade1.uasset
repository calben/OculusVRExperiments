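; Throwable grenade actor that can be picked up, armed and released, exploding on a timed fuse.
; Pickup disables GrabSphere physics and snaps the grenade to the holder, while Drop restores physics and detaches it in world space.
; IndexPressed arms it and records the start time.
; Tick polls the elapsed time and, after three seconds, spawns an enlarged ProjectileImpactBlast at GrabSphere once, then destroys the grenade.
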(event `self.ReceiveTick`
  (params (DeltaSeconds :type "Float (single-precision)"))
  (bind (_returnvalue_location _returnvalue_rotation) (`KismetMathLibrary.BreakTransform` (`SceneComponent.K2_GetComponentToWorld` (`self.GrabSphere`))))
  (if (`self.Activated`)
    (if (>= (- (`KismetSystemLibrary.GetGameTimeInSeconds`) (`self.ActivationStartTime`)) 3.0)
      (`/Engine/EditorBlueprintResources/StandardMacros.DoOnce` false
        (:`Completed`
          (`|SpawnActorFromClass` "/Game/Blueprints/ProjectileImpactBlast.ProjectileImpactBlast_C" (`KismetMathLibrary.MakeTransform` _returnvalue_location _returnvalue_rotation (3.0 3.0 3.0)) "Undefined" "OverrideRootScale")
          (`self.K2_DestroyActor`))))))

(event `/Game/VirtualRealityBP/Blueprints/IndexInterface.IndexPressed`
  (set `self.Activated` true)
  (set `self.ActivationStartTime` (`KismetSystemLibrary.GetGameTimeInSeconds`)))

(event `/Game/VirtualRealityBP/Blueprints/PickupActorInterface.Pickup`
  (params (AttachTo :type "SceneComponent Object Reference"))
  (`PrimitiveComponent.SetSimulatePhysics` (`self.GrabSphere`) false)
  (`self.K2_AttachRootComponentTo` AttachTo "None" "SnapToTarget"))

(event `/Game/VirtualRealityBP/Blueprints/PickupActorInterface.Drop`
  (`PrimitiveComponent.SetSimulatePhysics` (`self.GrabSphere`) true)
  (`self.K2_DetachFromActor` "KeepWorld" "KeepWorld"))

(fn `UserConstructionScript`)